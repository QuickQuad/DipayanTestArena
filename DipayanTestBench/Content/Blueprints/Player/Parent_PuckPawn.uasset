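; Base puck pawn that a local player controls, intended by its name as a parent for puck pawn variants.
; On BeginPlay it waits briefly, then has the player controller at PlayerControllerID possess it and enables input from that controller.
; MoveUp and MoveRight axis inputs feed the FloatingPawnMovement component along world X and Y respectively.
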(event EventBeginPlay
  (bind _playercontrollerid (Variables|Default|GetPlayerControllerID))
  (bind _returnvalue (Game|GetPlayerController _playercontrollerid))
  (Utilities|FlowControl|Delay 0.1)
  (Pawn|Possess _returnvalue self)
  (Input|EnableInput _returnvalue))

(event Input|AxisEvents|InputAxisMoveUp
  (params (AxisValue :type Float%20%28single-precision%29))
  (Class|PawnMovementComponent|AddInputVector (Variables|Default|GetFloatingPawnMovement) (Math|Vector|MakeVector AxisValue 0.0 0.0) false))

(event Input|AxisEvents|InputAxisMoveRight
  (params (AxisValue :type Float%20%28single-precision%29))
  (Class|PawnMovementComponent|AddInputVector (Variables|Default|GetFloatingPawnMovement) (Math|Vector|MakeVector 0.0 AxisValue 0.0) false))

(fn ConstructionScript)